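; Wraith character with a warp jump that serves as both wall jump and charge-limited air jump.
; In the air, a capsule trace along the last jump direction finds walls, launching the character along input or mirrored off the surface; without a hit, it spends a pip.
; A timeline eases velocity into each warp jump.
; Landing starts a looping timer that refills pips, and BeginPlay adds the pip widget.
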(event `ServerWJCapsuleTrace`
  (`self.WJCapsuleTrace`))

(event `WJWindDown`
  (params (InputVelocity :type "Vector Structure"))
  (bind (_direction _warp) (`Timeline|Timeline_0` :!via `PlayFromStart`)
    (:`Update`
      (`self.WJVelocityLerp` InputVelocity _warp))
    (:`Finished`
      (`KismetSystemLibrary.PrintString` "Jumped"))))

(event `WJ`
  (bind _returnvalue (* (`KismetMathLibrary.MakeVector` (.x (`self.GetLastMovementInputVector`)) (.y (`self.GetLastMovementInputVector`)) (`self.ZScale`)) (`self.WarpJumpMultiplier`)))
  ;[1 1 1] WJ
  (if (`NavMovementComponent.IsFalling` (`self.CharacterMovement`)) :!label _label
    (if (`self.Jumped`)
      (`/Engine/EditorBlueprintResources/ActorMacros.Switch Has Authority`
        (:`Authority`
          (`self.WJCapsuleTrace`))
        (:`Remote`
          (`self.ServerWJCapsuleTrace`)))
      (if (`self.CapsuleTraceHit`)
        (if (or (!= (`self.GetInputAxisValue`) 0.0) (!= (`self.GetInputAxisValue`) 0.0))
          (`self.WJWindDown` _returnvalue)
          (else
            (`self.WJWindDown` (`self.MirrorVelocity`))))
        (else
          (if (> (`self.Pips`) 0)
            (`self.WJWindDown` (+ _returnvalue (* (`MovementComponent.Velocity` (`self.CharacterMovement`)) (`self.WJScale`))))
            (`self.ServerCountPip`))
          (if (<= (`self.Pips`) 0)
            (set `self.Jumped` false))))
      (set `self.WJDirection` (`MovementComponent.Velocity` (`self.CharacterMovement`))))
    (else
      (`self.BaseJump` (0.0 0.0 750.0))
      (set `self.WJDirection` (`self.GetLastMovementInputVector`))
      (set `self.Jumped` true))))

(event `self.ReceiveBeginPlay`
  ;[1 1 1] BeginPlay
  (`parent.ReceiveBeginPlay`)
  (bind _returnvalue (`|CreateWidget` "/Game/NewStreak/Core/CoreUIandEffects/BP_Pips.BP_Pips_C"))
  (`UserWidget.AddToViewport` _returnvalue 0))

(event `ServerCountPip`
  (set `self.Pips` (- (`self.Pips`) 1)))

(event `InputAction|Jump`
  (params (Key :type "Key Structure"))
  (:`Pressed`
    (`/Engine/EditorBlueprintResources/ActorMacros.Switch Has Authority`
      (:`Authority`
        (goto _label))
      (:`Remote`
        (`self.WJ`)))))

(event `RegenTimer`
  (bind _returnvalue (`KismetSystemLibrary.K2_SetTimerDelegate` (delegate `PipRegen`) 0.25 true)))

(event `self.OnLanded`
  (params (Hit :type "HitResult Structure (by ref)"))
  (`self.RegenTimer`))

(event `PipRegen`
  (`self.PipRegenFunc` (stale `RegenTimer` _returnvalue)))

(event `InputAction|MoveAbility`
  (params (Key :type "Key Structure"))
  ;[1 1 1] MoveAbility
  (:`Pressed`
    (bind _returnvalue (`GameplayStatics.GetCurrentLevelName` true))
    (`KismetSystemLibrary.PrintString` _returnvalue)))

(fn `CountPip`
  (set `self.Pips` (- (`self.Pips`) 1)))

(fn `PipRegenFunc`
  (params (TimerHandle :type "TimerHandle Structure"))
  (if (not (`NavMovementComponent.IsFalling` (`self.CharacterMovement`)))
    (set `self.Pips` (+ (`self.Pips`) 1))
    (if (not (< (`self.Pips`) (`self.TotalPips`)))
      (`KismetSystemLibrary.K2_ClearAndInvalidateTimerHandle` TimerHandle))))

(fn `UserConstructionScript`
  (`parent.UserConstructionScript`))

(fn `WallJump`)

(fn `WJBasic`
  (if (<= (`self.Pips`) 0)
    (set `self.Jumped` false))
  (return))

(fn `WJCapsuleTrace`
  (bind _returnvalue (`SceneComponent.K2_GetComponentLocation` (`self.FirstPersonCamera`)))
  (bind (_returnvalue_x _returnvalue_y) (`KismetMathLibrary.BreakVector` (`KismetMathLibrary.Normal` (`self.WJDirection`))))
  (bind _returnvalue_2 (+ _returnvalue (* (`KismetMathLibrary.MakeVector` _returnvalue_x _returnvalue_y) (`self.LTLength`))))
  (bind (_outhit _returnvalue_3) (`KismetSystemLibrary.CapsuleTraceSingle` :`Start` _returnvalue :`End` _returnvalue_2 :`Radius` 65.0 :`HalfHeight` 122.0 :`TraceChannel` "TraceTypeQuery2" :`DrawDebugType` "ForDuration"))
  (set `self.CapsuleTraceHit` _returnvalue_3)
  (set `self.MirrorVelocity` (* (`KismetMathLibrary.MakeVector` (.x (`KismetMathLibrary.Normal` (`KismetMathLibrary.MirrorVectorByNormal` (- _returnvalue_2 _returnvalue) (`.ImpactNormal` (`GameplayStatics.BreakHitResult` _outhit))))) (.y (`KismetMathLibrary.Normal` (`KismetMathLibrary.MirrorVectorByNormal` (- _returnvalue_2 _returnvalue) (`.ImpactNormal` (`GameplayStatics.BreakHitResult` _outhit))))) (`self.ZScale`)) (`self.WarpJumpMultiplier`))))

(fn `WJVelocityLerp`
  (params (EndVelocity :type "Vector Structure") (Alpha :type "Float (double-precision)"))
  (bind _charactermovement (`self.CharacterMovement`))
  (set `MovementComponent.Velocity` (`KismetMathLibrary.VLerp` (`MovementComponent.Velocity` _charactermovement) EndVelocity Alpha) _charactermovement))