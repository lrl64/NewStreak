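; Enforcer playable character with a double jump and a fuel-powered movement ability, shown alongside a fuel HUD widget created at BeginPlay.
; MoveAbility presses toggle low gravity, multiplied walk speed and acceleration, and authority-only faster weapon fire and reload with a distortion flag.
; Looping timers drain fuel while active and regenerate it afterwards, with an empty tank forcing the ability off.
; NewGravity, ResetGravity and MoveCheck are not called within this Blueprint.
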(event `self.ReceiveBeginPlay`
  ;[1 1 1] BeginPlay
  (`parent.ReceiveBeginPlay`)
  (bind _returnvalue (`|CreateWidget` "/Game/NewStreak/Core/CoreUIandEffects/BP_Fuel.BP_Fuel_C"))
  (`UserWidget.AddToViewport` _returnvalue 0))

(event `InputAction|Jump`
  (params (Key :type "Key Structure"))
  ;[1 1 1] Jumping
  (:`Pressed`
    (bind _counter (`/Engine/EditorBlueprintResources/StandardMacros.Do N` 2 :!label _label)
      (:`Exit`
        (switch `int` _counter
          (:`1`
            _)
          (:`2`
            _))
        (bind _launchvector (`self.GetZLaunchFromJumpDuration` 0.75))
        (`self.BaseJump` _launchvector)))))

(event `self.OnLanded`
  (params (Hit :type "HitResult Structure (by ref)"))
  ;[1 1 1] Jumping
  (goto _label :!via `Reset`))

(event `InputAction|MoveAbility`
  (params (Key :type "Key Structure"))
  ;[1 1 1] MoveAbility
  (:`Pressed`
    (if (> (`self.PercFuel`) 0.0)
      (set `CharacterMovementComponent.GravityScale` 0.3 (`self.CharacterMovement`))
      (bind _counter (`/Engine/EditorBlueprintResources/StandardMacros.Do N` 2 :!label _label_2)
        (:`Exit`
          (switch `int` _counter
            (:`1`
              (`|ExecutionSequence`
                (:`then_0`
                  (`KismetSystemLibrary.K2_ClearAndInvalidateTimerHandle` (stale _returnvalue_2) :!label _label_3))
                (:`then_1`
                  (bind _returnvalue (`KismetSystemLibrary.K2_SetTimerDelegate` (delegate `EatFuel`) 0.022 true)))
                (:`then_2`
                  (`self.Sprinting`)
                  (`self.BuffWeaponSpeedAndReload`))))
            (:`2`
              (`|ExecutionSequence` :!label _label_4
                (:`then_0`
                  (`KismetSystemLibrary.K2_ClearAndInvalidateTimerHandle` _returnvalue))
                (:`then_1`
                  (bind _returnvalue_2 (`KismetSystemLibrary.K2_SetTimerDelegate` (delegate `RegenFuel`) 0.035 true)))
                (:`then_2`
                  (goto _label_2 :!via `Reset`))
                (:`then_3`
                  (`self.ResetMovement`)
                  (set `CharacterMovementComponent.GravityScale` 1.0 (`self.CharacterMovement`))
                  (`self.ResetWeaponSpeedAndReload`))))))))))

(event `EatFuel`
  ;[1 1 1] MoveAbility
  (bind _output_get (set `self.PercFuel` (- (`self.PercFuel`) 0.005)))
  (if (<= _output_get 0.0)
    (goto _label_4)))

(event `RegenFuel`
  ;[1 1 1] MoveAbility
  (bind _output_get (set `self.PercFuel` (+ (`self.PercFuel`) 0.005)))
  (if (>= _output_get 1.0)
    (goto _label_3)))

(fn `BuffWeaponSpeedAndReload`
  (bind _sprintmultiplier (`self.SprintMultiplier`))
  (`/Engine/EditorBlueprintResources/ActorMacros.Switch Has Authority`
    (:`Authority`
      (for _index (range (`KismetArrayLibrary.Array_Length` (`self.Weapons`)))
        (bind _output (`|GetArrayItem` (`self.Weapons`) _index))
        (set `/Game/NewStreak/Core/Weapons/BP_FiringWeaponBase.FireRate` (/ (`/Game/NewStreak/Core/Weapons/BP_FiringWeaponBase.FireRate` _output) _sprintmultiplier) _output)
        (set `/Game/NewStreak/Core/Weapons/BP_FiringWeaponBase.ReloadTime` (/ (`/Game/NewStreak/Core/Weapons/BP_FiringWeaponBase.ReloadTime` _output) _sprintmultiplier) _output)
        (set `self.DistortionActive?` true)))))

(fn `MoveCheck`
  (if (> (`self.PercFuel`) 0.0)
    (bind _counter (`/Engine/EditorBlueprintResources/StandardMacros.Do N` 2 :!label _label)
      (:`Exit`
        (switch `int` _counter
          (:`1`
            (set `self.IsMoving` true))
          (:`2`
            (set `self.IsMoving` false)
            (set `self.StartCooldown` true)
            (goto _label :!via `Reset`)))))))

(fn `NewGravity`
  (set `CharacterMovementComponent.GravityScale` 0.6 (`self.CharacterMovement`)))

(fn `ResetGravity`
  (set `CharacterMovementComponent.GravityScale` 1.0 (`Character.CharacterMovement` (`GameplayStatics.GetPlayerCharacter` 0))))

(fn `ResetMovement`
  (bind _charactermovement (`self.CharacterMovement`))
  (set `CharacterMovementComponent.MaxWalkSpeed` (`self.DefaultMaxSpeed`) _charactermovement)
  (set `CharacterMovementComponent.MaxAcceleration` (`self.DefAccel`) _charactermovement))

(fn `ResetWeaponSpeedAndReload`
  (bind _sprintmultiplier (`self.SprintMultiplier`))
  (`/Engine/EditorBlueprintResources/ActorMacros.Switch Has Authority`
    (:`Authority`
      (for _index (range (`KismetArrayLibrary.Array_Length` (`self.Weapons`)))
        (bind _output (`|GetArrayItem` (`self.Weapons`) _index))
        (set `/Game/NewStreak/Core/Weapons/BP_FiringWeaponBase.FireRate` (* (`/Game/NewStreak/Core/Weapons/BP_FiringWeaponBase.FireRate` _output) _sprintmultiplier) _output)
        (set `/Game/NewStreak/Core/Weapons/BP_FiringWeaponBase.ReloadTime` (* (`/Game/NewStreak/Core/Weapons/BP_FiringWeaponBase.ReloadTime` _output) _sprintmultiplier) _output)
        (set `self.DistortionActive?` false)))))

(fn `Sprinting`
  (bind _sprintmultiplier (`self.SprintMultiplier`))
  (bind _charactermovement (`self.CharacterMovement`))
  (bind _returnvalue (`CharacterMovementComponent.GetMaxAcceleration` _charactermovement))
  (bind _maxwalkspeed (`CharacterMovementComponent.MaxWalkSpeed` _charactermovement))
  (set `self.DefaultMaxSpeed` _maxwalkspeed)
  (set `CharacterMovementComponent.MaxWalkSpeed` (* _maxwalkspeed _sprintmultiplier) _charactermovement)
  (set `self.DefAccel` _returnvalue)
  (set `CharacterMovementComponent.MaxAcceleration` (* _sprintmultiplier _returnvalue) _charactermovement))

(fn `UserConstructionScript`
  (`parent.UserConstructionScript`))