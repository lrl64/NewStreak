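; Gunslinger player character with a directional warp dash, a mid-air warp jump and a thrown tactical knife.
; Both warps use timelines to lerp velocity up then down, shake the camera, and spend dash pips that looping timers refill.
; The knife spawns from the camera only when no other exists and expires after 10 seconds; its impulse branch is disconnected.
; Actions route through authority switches and Server-prefixed events for replication.
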(event `InputAction|Ability1`
  (params (Key :type "Key Structure")))

(event `ServerTacImpulse`
  (params (Target :type "PrimitiveComponent Object Reference"))
  (`self.TacImpulse` Target))

(event `InputAction|Ability2`
  (params (Key :type "Key Structure"))
  (:`Pressed`
    (`self.ServerAbility2`)))

(event `ServerAbility2`
  (bind _outactors (`GameplayStatics.GetAllActorsOfClass` "/Game/NewStreak/Blueprints/Characters/Gunslinger/BP_GSProjectile.BP_GSProjectile_C"))
  (if (not (> (`KismetArrayLibrary.Array_Length` _outactors) 0))
    (bind (_returnvalue _materialsphere1) (`self.TacKnife`))
    (`KismetSystemLibrary.Delay` 10.0)
    (`/Engine/EditorBlueprintResources/StandardMacros.IsValid` _returnvalue
      (:`Is Valid`
        (`self.K2_DestroyActor` _returnvalue)
        (`KismetSystemLibrary.PrintString` "Knife Ready")))))

(event `ServerWJVelocityWindDown`
  (params (Alpha :type "Float (double-precision)"))
  ;[1 1 1] Replication Events
  (`self.WJVelocityWindDown` Alpha))

(event `ServerWJVelocityUpdate`
  (params (Alpha :type "Float (double-precision)"))
  ;[1 1 1] Replication Events
  (`self.WJVelocityUpdate` Alpha))

(event `InputAction|Blindfire`
  (params (Key :type "Key Structure"))
  ;[1 1 1] Blindfire
  (:`Pressed`
    (`KismetSystemLibrary.PrintString` (`KismetStringLibrary.Conv_VectorToString` (`self.K2_GetActorLocation`)))))

(event `ServerBaseJump`
  ;[1 1 1] Replication Events
  (`self.BaseJump` (`self.GSJump`)))

(event `self.ReceiveBeginPlay`
  ;[1 1 1] BeginPlay
  (`parent.ReceiveBeginPlay`)
  (bind _returnvalue (`|CreateWidget` "/Game/NewStreak/Core/CoreUIandEffects/BP_DashPips.BP_DashPips_C"))
  (`UserWidget.AddToViewport` _returnvalue 0))

(event `ServerWarpJumpPreamble`
  ;[1 1 1] Replication Events
  (`self.WarpJumpPreamble`))

(event `ServerWarpPreamble`
  ;[1 1 1] Replication Events
  (`self.WarpPreamble`))

(event `ServerWarpSetSpeed`
  (params (InputVelocity :type "Vector Structure"))
  ;[1 1 1] Replication Events
  (`self.WarpSetSpeed` InputVelocity))

(event `JumpEvent`
  ;[1 1 1] WarpJump
  (if (> (`self.Pips`) 0) :!label _label
    (`/Engine/EditorBlueprintResources/ActorMacros.Switch Has Authority`
      (:`Authority`
        (`self.WarpJumpPreamble`)
        (bind (_direction _warpwindup) (`Timeline|WarpJumpInitial` :!via `PlayFromStart` :!label _label_2)
          (:`Update`
            (`/Engine/EditorBlueprintResources/ActorMacros.Switch Has Authority`
              (:`Authority`
                (`self.WJVelocityUpdate` _warpwindup))
              (:`Remote`
                (`self.ServerWJVelocityUpdate` _warpwindup))))
          (:`Finished`
            (`self.ServerCameraShake`)
            (set `self.WarpJumpResetSpeed` (`MovementComponent.Velocity` (`self.CharacterMovement`)))
            (bind (_direction_2 _warp) (`Timeline|WarpJumpSlowDown` :!via `PlayFromStart`)
              (:`Update`
                (`/Engine/EditorBlueprintResources/ActorMacros.Switch Has Authority`
                  (:`Authority`
                    (`self.WJVelocityWindDown` _warp))
                  (:`Remote`
                    (`self.ServerWJVelocityWindDown` _warp))))
              (:`Finished`
                (`KismetSystemLibrary.PrintString` "Warped")
                (`self.ServerCountPip`)
                (if (`self.WarpCooldownActive`)
                  (bind _returnvalue (`KismetSystemLibrary.K2_SetTimerDelegate` (delegate `PipRegen`) 0.0225 true))))))))
      (:`Remote`
        (`self.ServerWarpJumpPreamble`)
        (goto _label_2 :!via `PlayFromStart`)))))

(event `ServerVelocityWindDown`
  (params (Alpha :type "Float (double-precision)"))
  ;[1 1 1] Replication Events
  (`self.VelocityWindDown` Alpha))

(event `InputAction|Jump`
  (params (Key :type "Key Structure"))
  ;[1 1 1] WarpJump
  (:`Pressed`
    (if (`NavMovementComponent.IsFalling` (`self.CharacterMovement`))
      (`/Engine/EditorBlueprintResources/ActorMacros.Switch Has Authority`
        (:`Authority`
          (goto _label))
        (:`Remote`
          (`self.JumpEvent`)))
      (else
        (`/Engine/EditorBlueprintResources/ActorMacros.Switch Has Authority`
          (:`Authority`
            (`self.BaseJump` (`self.GSJump`)))
          (:`Remote`
            (`self.ServerBaseJump`)))))))

(event `ServerCameraShake`
  ;[1 1 1] Replication Events
  (`GameplayStatics.PlayWorldCameraShake` "/Game/NewStreak/Core/CoreUIandEffects/BP_WarpShake.BP_WarpShake_C" (`self.K2_GetActorLocation`) 0.0 500.0))

(event `PipRegen`
  ;[1 1 1] WarpJump
  (`self.ServerPipCooldown` (stale `JumpEvent` _returnvalue)))

(event `ServerPipCooldown`
  (params (Handle :type "TimerHandle Structure"))
  ;[1 1 1] Replication Events
  (`self.PipCooldown` Handle))

(event `ServerVelocityUpdate`
  (params (Alpha :type "Float (double-precision)"))
  ;[1 1 1] Replication Events
  (`self.VelocityUpdate` Alpha))

(event `ServerCountPip`
  ;[1 1 1] Replication Events
  (`self.CountPip`))

(event `ServerMoveAbility`
  ;[1 1 1] Warping
  (if (> (`self.Pips`) 0) :!label _label_3
    (`/Engine/EditorBlueprintResources/ActorMacros.Switch Has Authority`
      (:`Authority`
        (`self.WarpPreamble`)
        (bind (_direction _warpwindup) (`Timeline|WarpInitial` :!via `PlayFromStart` :!label _label_4)
          (:`Update`
            (`/Engine/EditorBlueprintResources/ActorMacros.Switch Has Authority`
              (:`Authority`
                (`self.VelocityUpdate` _warpwindup))
              (:`Remote`
                (`self.ServerVelocityUpdate` _warpwindup))))
          (:`Finished`
            (`self.ServerCameraShake`)
            (set `self.WarpResetSpeed` (`MovementComponent.Velocity` (`self.CharacterMovement`)))
            (bind (_direction_2 _warp) (`Timeline|WarpSlowDown` :!via `PlayFromStart`)
              (:`Update`
                (`/Engine/EditorBlueprintResources/ActorMacros.Switch Has Authority`
                  (:`Authority`
                    (`self.VelocityWindDown` _warp))
                  (:`Remote`
                    (`self.ServerVelocityWindDown` _warp))))
              (:`Finished`
                (`KismetSystemLibrary.PrintString` "Warped")
                (`self.ServerCountPip`)
                (bind _returnvalue (`KismetSystemLibrary.K2_SetTimerDelegate` (delegate `PipRegen1`) 0.0225 true)))))))
      (:`Remote`
        (`self.ServerWarpPreamble`)
        (goto _label_4 :!via `PlayFromStart`)))))

(event `InputAction|MoveAbility`
  (params (Key :type "Key Structure"))
  ;[1 1 1] Warping
  (:`Pressed`
    (`/Engine/EditorBlueprintResources/ActorMacros.Switch Has Authority`
      (:`Authority`
        (goto _label_3))
      (:`Remote`
        (`self.ServerMoveAbility`)))))

(event `PipRegen1`
  ;[1 1 1] Warping
  (`self.ServerPipCooldown` (stale `ServerMoveAbility` _returnvalue)))

(fn `CountPip`
  (bind _output_get (set `self.Pips` (`KismetMathLibrary.Clamp` (- (`self.Pips`) 1) 0 (`self.TotalPips`))))
  (set `self.WarpCooldownActive` (< _output_get (`self.TotalPips`))))

(fn `PipCooldown`
  (params (Handle :type "TimerHandle Structure"))
  ;[1 1 1] Loop until condition is true
  (set `self.DashRegen` (+ (`self.DashRegen`) 0.005))
  (if (>= (`self.DashRegen`) 1.0)
    (set `self.Pips` (`KismetMathLibrary.Clamp` (+ (`self.Pips`) 1) 0 (`self.TotalPips`)))
    (set `self.DashRegen` 0.0)
    (if (>= (`self.Pips`) (`self.TotalPips`))
      (`KismetSystemLibrary.K2_ClearAndInvalidateTimerHandle` Handle))))

(fn `TacImpulse`
  (params (Target :type "PrimitiveComponent Object Reference"))
  (`PrimitiveComponent.AddImpulse` Target (* (`SceneComponent.GetForwardVector` (`self.FirstPersonCamera`)) (`self.ProjectileSpeed`)) "None" true))

(fn `TacKnife`
  (returns (ReturnValue :type "/Game/NewStreak/Blueprints/Characters/Gunslinger/BP_GSProjectile Object Reference") (MaterialSphere1 :type "StaticMeshComponent Object Reference"))
  (bind _firstpersoncamera (`self.FirstPersonCamera`))
  (bind _returnvalue (`|SpawnActorFromClass` "/Game/NewStreak/Blueprints/Characters/Gunslinger/BP_GSProjectile.BP_GSProjectile_C" (`KismetMathLibrary.MakeTransform` (+ (`SceneComponent.K2_GetComponentLocation` _firstpersoncamera) (* (`SceneComponent.GetForwardVector` _firstpersoncamera) 100.0)) (`self.GetControlRotation`) (0.5 0.5 0.5)) "AlwaysSpawn" "OverrideRootScale" null (`GameplayStatics.GetPlayerCharacter` 0)))
  (return _returnvalue null))

(fn `UserConstructionScript`
  (`parent.UserConstructionScript`))

(fn `VelocityUpdate`
  (params (Alpha :type "Float (double-precision)"))
  (set `MovementComponent.Velocity` (`KismetMathLibrary.VLerp` (`self.WarpResetSpeed`) (`self.WarpFinalSpeed`) Alpha) (`self.CharacterMovement`)))

(fn `VelocityWindDown`
  (params (Alpha :type "Float (double-precision)"))
  (bind _warpresetspeed (`self.WarpResetSpeed`))
  (set `MovementComponent.Velocity` (`KismetMathLibrary.VLerp` _warpresetspeed (* _warpresetspeed (`self.WarpWindDown`)) Alpha) (`self.CharacterMovement`)))

(fn `WarpJumpPreamble`
  (set `self.WarpJumpFinalSpeed` (* (`self.WarpJumpInput`) (`self.WarpJumpMultiplier`)))
  (set `self.WarpJumpResetSpeed` (`MovementComponent.Velocity` (`self.CharacterMovement`)))
  (`CharacterMovementComponent.AddImpulse` (`self.CharacterMovement`) (0.0 0.0 50.0) true))

(fn `WarpPreamble`
  (bind _returnvalue (`self.GetInputAxisValue`))
  (bind _charactermovement (`self.CharacterMovement`))
  (`self.ServerSetDirection`)
  (`KismetSystemLibrary.PrintString` (`KismetStringLibrary.Conv_DoubleToString` _returnvalue))
  (if (or (!= _returnvalue 0.0) (!= (`self.GetInputAxisValue`) 0.0))
    (set `self.WarpFinalSpeed` (* (+ (* (`self.Direction1`) (`self.GetInputAxisValue`)) (* (`self.Direction2`) (`self.GetInputAxisValue`))) (`self.WarpMultiplier`)))
    (else
      (set `self.WarpFinalSpeed` (* (`self.Direction1`) (`self.WarpMultiplier`)))))
  (set `self.WarpResetSpeed` (`MovementComponent.Velocity` _charactermovement))
  (`CharacterMovementComponent.AddImpulse` _charactermovement (0.0 0.0 50.0) true))

(fn `WarpSetSpeed`
  (params (InputVelocity :type "Vector Structure"))
  (set `self.WarpFinalSpeed` (* InputVelocity (`self.WarpMultiplier`))))

(fn `WJVelocityUpdate`
  (params (Alpha :type "Float (double-precision)"))
  (set `MovementComponent.Velocity` (`KismetMathLibrary.VLerp` (`self.WarpJumpResetSpeed`) (`self.WarpJumpFinalSpeed`) Alpha) (`self.CharacterMovement`)))

(fn `WJVelocityWindDown`
  (params (Alpha :type "Float (double-precision)"))
  (bind _warpjumpresetspeed (`self.WarpJumpResetSpeed`))
  (set `MovementComponent.Velocity` (`KismetMathLibrary.VLerp` _warpjumpresetspeed (* _warpjumpresetspeed (`self.WarpJumpWindDown`)) Alpha) (`self.CharacterMovement`)))