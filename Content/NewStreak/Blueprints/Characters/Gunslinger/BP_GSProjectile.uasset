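; BP_GSProjectile is a Gunslinger projectile, apparently a thrown knife, that deals very heavy damage to whatever it hits.
; On a sphere component hit it applies damage credited to its instigator, stops its movement and attaches to the struck component, keeping its world transform.
; It then hides its sphere mesh, waits out a Cooldown delay, destroys itself and prints a "Knife Ready" debug message.
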(event `self.Sphere.OnComponentHit`
  (params (HitComponent :type "PrimitiveComponent Object Reference") (OtherActor :type "Actor Object Reference") (OtherComp :type "PrimitiveComponent Object Reference") (NormalImpulse :type "Vector Structure") (Hit :type "HitResult Structure (by ref)"))
  (`GameplayStatics.ApplyDamage` OtherActor 1000.0 (`self.GetInstigatorController`) self)
  (`MovementComponent.StopMovementImmediately` (`self.ProjectileMovement`))
  (`self.K2_AttachToComponent` OtherComp "None" "KeepWorld" "KeepWorld" "KeepWorld")
  (`SceneComponent.SetVisibility` (`self.MaterialSphere1`) false false)
  (`KismetSystemLibrary.Delay` (`self.Cooldown`))
  (`self.K2_DestroyActor`)
  (`KismetSystemLibrary.PrintString` "Knife Ready"))

(fn `UserConstructionScript`)