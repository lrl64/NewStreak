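; BP_MenuCharacterShowcase is a menu display that shows two randomly picked characters from a roster of seven, each looping a third-person idle animation.
; On BeginPlay, a stored random index selects the first skeletal mesh, and a second switch sets the other mesh.
; A random check against the first index loops back through the sequence on a match, but the second pick rolls separately, so duplicates remain possible.
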(event `self.ReceiveBeginPlay`
  (bind _returnvalue (`KismetMathLibrary.RandomInteger` 7))
  (bind _skeletalmesh1 (`self.SkeletalMesh1`))
  (bind _skeletalmesh (`self.SkeletalMesh`))
  (set `self.Switch` (`KismetMathLibrary.RandomInteger` 7))
  (`|ExecutionSequence` :!label _label
    (:`then_0`
      (switch `int` (`self.Switch`)
        (:`0`
          (set `self.TheChosen` "/Game/NewStreak/Blueprints/Characters/Assassin/SK_Assassin.SK_Assassin"))
        (:`1`
          (set `self.TheChosen` "/Game/NewStreak/Blueprints/Characters/Enforcer/SK_Enforcer.SK_Enforcer"))
        (:`2`
          (set `self.TheChosen` "/Game/NewStreak/Blueprints/Characters/Gunslinger/SK_Gunslinger.SK_Gunslinger"))
        (:`3`
          (set `self.TheChosen` "/Game/NewStreak/Blueprints/Characters/Harrier/SK_Harrier.SK_Harrier"))
        (:`4`
          (set `self.TheChosen` "/Game/NewStreak/Blueprints/Characters/Juggernaut/SK_Juggs.SK_Juggs"))
        (:`5`
          (set `self.TheChosen` "/Game/NewStreak/Blueprints/Characters/Vanguard/SK_Vanguard.SK_Vanguard"))
        (:`6`
          (set `self.TheChosen` "/Game/NewStreak/Blueprints/Characters/Wraith/SK_Wraith.SK_Wraith")))
      (`SkinnedMeshComponent.SetSkinnedAssetAndUpdate` _skeletalmesh (`self.TheChosen`) true)
      (`SkeletalMeshComponent.PlayAnimation` _skeletalmesh "/Game/NewStreak/3rdPartyLibrariesImports/3rdPersonTemplate/Mannequin/Animations/ThirdPersonIdle.ThirdPersonIdle" true))
    (:`then_1`
      (if (== _returnvalue (`self.Switch`))
        (goto _label)
        (else
          (switch `int` _returnvalue
            (:`0`
              (set `self.TheSecondChosen` "/Game/NewStreak/Blueprints/Characters/Assassin/SK_Assassin.SK_Assassin"))
            (:`1`
              (set `self.TheSecondChosen` "/Game/NewStreak/Blueprints/Characters/Enforcer/SK_Enforcer.SK_Enforcer"))
            (:`2`
              (set `self.TheSecondChosen` "/Game/NewStreak/Blueprints/Characters/Gunslinger/SK_Gunslinger.SK_Gunslinger"))
            (:`3`
              (set `self.TheSecondChosen` "/Game/NewStreak/Blueprints/Characters/Harrier/SK_Harrier.SK_Harrier"))
            (:`4`
              (set `self.TheSecondChosen` "/Game/NewStreak/Blueprints/Characters/Juggernaut/SK_Juggs.SK_Juggs"))
            (:`5`
              (set `self.TheSecondChosen` "/Game/NewStreak/Blueprints/Characters/Vanguard/SK_Vanguard.SK_Vanguard"))
            (:`6`
              (set `self.TheSecondChosen` "/Game/NewStreak/Blueprints/Characters/Wraith/SK_Wraith.SK_Wraith")))
          (`SkinnedMeshComponent.SetSkinnedAssetAndUpdate` _skeletalmesh1 (`self.TheSecondChosen`) true)
          (`SkeletalMeshComponent.PlayAnimation` _skeletalmesh1 "/Game/NewStreak/3rdPartyLibrariesImports/3rdPersonTemplate/Mannequin/Animations/ThirdPersonIdle.ThirdPersonIdle" true))))))

(fn `UserConstructionScript`)