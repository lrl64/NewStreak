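; BP_GravityVolume is a box trigger that scales gravity for any BP_FPSBaseCharacter inside it by LowGravScale.
; On begin overlap it stores the character's GravityScale and starts a looping timer that keeps applying the scaled value.
; On end overlap it restores the stored value and clears the timer, with debug prints on both events.
; It holds one stored gravity value and one timer handle, not per-character state.
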(event `self.Box.OnComponentBeginOverlap`
  (params (OverlappedComponent :type "PrimitiveComponent Object Reference") (OtherActor :type "Actor Object Reference") (OtherComp :type "PrimitiveComponent Object Reference") (OtherBodyIndex :type Integer) (bFromSweep :type Boolean) (SweepResult :type "HitResult Structure (by ref)"))
  (bind (_asbp_fpsbase_character _bsuccess) (cast `/Game/NewStreak/Core/Characters/BP_FPSBaseCharacter` OtherActor :!pure true))
  (if _bsuccess
    (set `self.InitialGrav` (`CharacterMovementComponent.GravityScale` (`Character.CharacterMovement` _asbp_fpsbase_character)))
    (`KismetSystemLibrary.PrintString` "Hello")
    (bind _returnvalue (`KismetSystemLibrary.K2_SetTimerDelegate` (delegate `GravTimer`) 0.1 true))))

(event `GravTimer`
  (set `CharacterMovementComponent.GravityScale` (* (`self.InitialGrav`) (`self.LowGravScale`)) (`Character.CharacterMovement` (cast `/Game/NewStreak/Core/Characters/BP_FPSBaseCharacter` (stale `self.Box.OnComponentBeginOverlap` OtherActor) :!pure true))))

(event `self.Box.OnComponentEndOverlap`
  (params (OverlappedComponent :type "PrimitiveComponent Object Reference") (OtherActor :type "Actor Object Reference") (OtherComp :type "PrimitiveComponent Object Reference") (OtherBodyIndex :type Integer))
  (bind (_asbp_fpsbase_character _bsuccess) (cast `/Game/NewStreak/Core/Characters/BP_FPSBaseCharacter` OtherActor :!pure true))
  (if _bsuccess
    (`KismetSystemLibrary.PrintString` "End Overlap")
    (set `CharacterMovementComponent.GravityScale` (`self.InitialGrav`) (`Character.CharacterMovement` _asbp_fpsbase_character))
    (`KismetSystemLibrary.K2_ClearAndInvalidateTimerHandle` (stale `self.Box.OnComponentBeginOverlap` _returnvalue))))

(fn `UserConstructionScript`)