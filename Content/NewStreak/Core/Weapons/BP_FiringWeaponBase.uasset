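; Base weapon Blueprint for firearms, handling firing checks, ammo, reload state and cosmetic feedback, with no hit or damage logic.
; OnFire requires the owner's Firing flag, ammo, durability and no active reload, then decrements ammo and triggers sound, shake, montage and muzzle flashes on both Mesh and the owner's FPGun.
; ReloadDelay flags reloading, Reload refills and updates the ammo text.
; BeginFire, EndFire, no-ammo sound and reload animation are empty stubs.
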(event `OnFire`
  (params (CrosshairWorldSpace :type "Vector Structure"))
  (bind _muzzleflash (`self.MuzzleFlash`))
  (bind _owningcharacter (`self.OwningCharacter`))
  (if (`/Game/NewStreak/Core/Characters/BP_FPSBaseCharacter.Firing?` (`self.OwningCharacter`))
    (bind _canfire (`self.CanWeaponFire`))
    (bind _output_get (set `self.CanFire?` _canfire))
    (if _output_get
      (`self.DecrementAmmoCount`)
      (set `self.LastFired` (`GameplayStatics.GetTimeSeconds`))
      (`self.1PMuzzleFlash` _muzzleflash)
      (`self.MulticastMuzzleFlash` _muzzleflash)
      (`self.ServerFireSound` (`self.FireStartSound`))
      (`GameplayStatics.PlayWorldCameraShake` "/Game/NewStreak/Core/CoreUIandEffects/BP_WeaponCameraShake.BP_WeaponCameraShake_C" (`self.K2_GetActorLocation` _owningcharacter) 0.0 500.0)
      (`/Game/NewStreak/Core/Characters/BP_FPSBaseCharacter.ClientPlayAnimMontageWeapon` _owningcharacter)
      (else
        (`self.PlayNoAmmoSound`)))
    (else
      (set `self.CanFire?` false))))

(event `EndFire`)

(event `BeginFire`)

(event `1PMuzzleFlash`
  (params (MuzzleFlash :type "ParticleSystem Object Reference"))
  (`self.PlayMuzzleFlash` MuzzleFlash))

(event `MulticastMuzzleFlash`
  (params (MuzzleFlash :type "ParticleSystem Object Reference"))
  (`self.PlayMuzzleFlashOnServer` MuzzleFlash))

(event `ServerFireSound`
  (params (FireSound :type "SoundBase Object Reference"))
  (`self.PlayFireSound` FireSound))

(event `ServerReloadCheck`
  (`self.CanBeReloadedCheck`))

(event `ReloadDelay`
  (set `self.Reloading?` true)
  (`self.PlayReloadSound`)
  (`self.PlayReloadAnimation`))

(event `PlayReloadSound`
  (`self.ReloadSound`))

(fn `CanBeReloadedCheck`
  (if (> (- (`self.MaxAmmoCount`) (`self.AmmoCount`)) 0.0)
    (set `self.CanReload?` true)
    (else
      (set `self.CanReload?` false))))

(fn `CanWeaponFire`
  (returns (CanFire :type Boolean))
  (if (> (`self.AmmoCount`) 0.0)
    (if (> (`self.Durability`) 0.0)
      (if (`self.Reloading?`)
        _
        (else
          (return true)))))
  (return false))

(fn `DecrementAmmoCount`
  (bind _output_get (set `self.AmmoCount` (`KismetMathLibrary.FClamp` (- (`self.AmmoCount`) 1.0) 0.0 (`self.MaxAmmoCount`))))
  (set `self.RemaningAmmoDisplay` (`KismetTextLibrary.Conv_DoubleToText` _output_get "HalfToEven"))
  (`TextRenderComponent.K2_SetText` (`self.AmmoDisplay`) (`self.RemaningAmmoDisplay`)))

(fn `PlayFireSound`
  (params (FireSound :type "SoundBase Object Reference"))
  (`GameplayStatics.SpawnSoundAtLocation` FireSound (`SceneComponent.GetSocketLocation` (`self.Mesh`) (`self.MuzzleSocket`))))

(fn `PlayMuzzleFlash`
  (params (MuzzleFlash :type "ParticleSystem Object Reference"))
  (bind _muzzlesocket (`self.MuzzleSocket`))
  (bind _mesh (`self.Mesh`))
  (bind _returnvalue (`GameplayStatics.SpawnEmitterAtLocation` MuzzleFlash (`SceneComponent.GetSocketLocation` _mesh _muzzlesocket) (`SceneComponent.GetSocketRotation` _mesh _muzzlesocket) (0.07 0.07 0.07)))
  (`SceneComponent.K2_AttachToComponent` _returnvalue _mesh _muzzlesocket "SnapToTarget" "SnapToTarget" "SnapToTarget" true))

(fn `PlayMuzzleFlashOnServer`
  (params (MuzzleFlash :type "ParticleSystem Object Reference"))
  (bind _muzzlesocket (`self.MuzzleSocket`))
  (bind _fp_gun (`/Game/NewStreak/Core/Characters/BP_FPSBaseCharacter.FP_Gun` (`self.OwningCharacter`)))
  (bind _returnvalue (`GameplayStatics.SpawnEmitterAtLocation` MuzzleFlash (`SceneComponent.GetSocketLocation` _fp_gun _muzzlesocket) (`SceneComponent.GetSocketRotation` _fp_gun _muzzlesocket)))
  (`SceneComponent.K2_AttachToComponent` _returnvalue _fp_gun _muzzlesocket "SnapToTarget" "SnapToTarget" "SnapToTarget" true))

(fn `PlayNoAmmoSound`)

(fn `PlayReloadAnimation`)

(fn `Reload`
  (bind _ammocount (`self.AmmoCount`))
  (set `self.AmmoCount` (+ (- (`self.MaxAmmoCount`) _ammocount) _ammocount))
  (set `self.Reloading?` false)
  (set `self.CanReload?` false)
  (`TextRenderComponent.K2_SetText` (`self.AmmoDisplay`) (`KismetTextLibrary.Conv_DoubleToText` (`self.AmmoCount`) "HalfToEven")))

(fn `ReloadSound`
  (`GameplayStatics.PlaySoundAtLocation` (`self.ReloadSoundCue`) (`self.K2_GetActorLocation` self) (struct) 0.1 1.0 1.0))

(fn `UserConstructionScript`
  (bind _output_get (set `self.RemaningAmmoDisplay` (`KismetTextLibrary.Conv_DoubleToText` (`self.AmmoCount`) "HalfToEven")))
  (`TextRenderComponent.K2_SetText` (`self.AmmoDisplay`) _output_get))